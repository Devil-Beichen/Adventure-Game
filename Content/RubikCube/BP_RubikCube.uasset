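; Rubik's cube actor with eight pieces that turns its top or left layer 90 degrees, one turn at a time.
; Get caches the pieces and their RangeWarn marker positions; Get层 sorts them into layers against the actor origin and saves relative rotations.
; Timelines lerp world yaw or roll through nested rotation-by-piece loops, so the last saved rotation wins for every piece.
; Layers are rebuilt at construction and after each turn.
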(event `self.ReceiveBeginPlay`)

(event `self.ReceiveTick`
  (params (DeltaSeconds :type "Float (single-precision)")))

(event `上层旋转`
  (if (not (`self.在转`))
    (set `self.在转` true)
    (`self.Get`)
    (bind (_direction `_新建轨道_0`) (`Timeline|时间轴_0` :!via `PlayFromStart`)
      (:`Update`
        (for _array_element (`self.上Rotation`)
          (for _array_element_2 (`self.上层`)
            (bind _yaw (.yaw _array_element))
            (`SceneComponent.K2_SetWorldRotation` _array_element_2 (`KismetMathLibrary.MakeRotator` (.roll _array_element) (.pitch _array_element) (`KismetMathLibrary.Lerp` _yaw (+ _yaw 90.0) `_新建轨道_0`)) false false))))
      (:`Finished`
        (`self.Get`)
        (`self.Get 层`)
        (set `self.在转` false)))))

(event `左侧旋转`
  (if (not (`self.在转`))
    (set `self.在转` true)
    (`self.Get`)
    (bind (_direction `_新建轨道_0`) (`Timeline|时间轴_1` :!via `PlayFromStart`)
      (:`Update`
        (for _array_element (`self.左Rotation`)
          (for _array_element_2 (`self.左层`)
            (bind _roll (.roll _array_element))
            (`SceneComponent.K2_SetWorldRotation` _array_element_2 (`KismetMathLibrary.MakeRotator` (`KismetMathLibrary.Lerp` _roll (+ _roll 90.0) `_新建轨道_0`) (.pitch _array_element) (.yaw _array_element)) false false))))
      (:`Finished`
        (`self.Get`)
        (`self.Get 层`)
        (set `self.在转` false)))))

(fn `Get`
  (set `self.Get All Relative Location` (`|MakeArray` (`SceneComponent.K2_GetComponentLocation` (`self.RangeWarn1`)) (`SceneComponent.K2_GetComponentLocation` (`self.RangeWarn2`)) (`SceneComponent.K2_GetComponentLocation` (`self.RangeWarn3`)) (`SceneComponent.K2_GetComponentLocation` (`self.RangeWarn4`)) (`SceneComponent.K2_GetComponentLocation` (`self.RangeWarn5`)) (`SceneComponent.K2_GetComponentLocation` (`self.RangeWarn6`)) (`SceneComponent.K2_GetComponentLocation` (`self.RangeWarn7`)) (`SceneComponent.K2_GetComponentLocation` (`self.RangeWarn8`))))
  (set `self.Get All Range` (`|MakeArray` (`self.Scene1`) (`self.Scene2`) (`self.Scene3`) (`self.Scene4`) (`self.Scene5`) (`self.Scene6`) (`self.Scene7`) (`self.Scene8`))))

(fn `Get 层`
  (bind _returnvalue_x (`KismetMathLibrary.BreakVector` (`self.K2_GetActorLocation`)))
  (bind (_returnvalue_x_2 _returnvalue_y _returnvalue_z) (`KismetMathLibrary.BreakVector` (`self.K2_GetActorLocation`)))
  (`KismetArrayLibrary.Array_Clear` (`self.上Rotation`))
  (`KismetArrayLibrary.Array_Clear` (`self.左Rotation`))
  (`|ExecutionSequence`
    (:`then_0`
      (`KismetArrayLibrary.Array_Clear` (`self.上层`))
      (for (_array_element _array_index) (`self.Get All Relative Location`)
        (if (> (.z _array_element) _returnvalue_z)
          (bind _output (`|GetArrayItem` (`self.Get All Range`) _array_index))
          (`KismetArrayLibrary.Array_AddUnique` (`self.上层`) _output)
          (`KismetArrayLibrary.Array_Add` (`self.上Rotation`) (`SceneComponent.RelativeRotation` _output)))))
    (:`then_1`
      (`KismetArrayLibrary.Array_Clear` (`self.左层`))
      (for (_array_element_2 _array_index_2) (`self.Get All Relative Location`)
        (if (< (.x _array_element_2) _returnvalue_x)
          (bind _output_2 (`|GetArrayItem` (`self.Get All Range`) _array_index_2))
          (`KismetArrayLibrary.Array_AddUnique` (`self.左层`) _output_2)
          (`KismetArrayLibrary.Array_Add` (`self.左Rotation`) (`SceneComponent.RelativeRotation` _output_2)))))))

(fn `UserConstructionScript`
  (`self.Get`)
  (`self.Get 层`))

(fn `新函数_0`
  (for _ (range (`self.X`))
    (for _ (range (`self.Y`))
      (for _ (range (`self.Z`))
        _))))